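; BP_ThrowObject_Tukkomi is a short-lived "Tukkomi" thrown object that reports its outcome to its owner through ApplyDamage.
; If it survives half a second, it applies negative damage to its owner and destroys itself a tick later.
; Overlapping something with a different owner applies small positive damage to its own owner and destroys the other actor if it is a BP_Projectile.
; Such an overlap also destroys the object on the next tick.
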(event `self.ReceiveBeginPlay`
  (`parent.ReceiveBeginPlay`)
  (`KismetSystemLibrary.Delay` 0.5)
  (`GameplayStatics.ApplyDamage` (`self.GetOwner` self) -0.3 null self)
  (`KismetSystemLibrary.DelayUntilNextTick`)
  (`self.K2_DestroyActor`))

(event `self. .OnComponentBeginOverlap`
  (params (OverlappedComponent :type "PrimitiveComponent Object Reference") (OtherActor :type "Actor Object Reference") (OtherComp :type "PrimitiveComponent Object Reference") (OtherBodyIndex :type Integer) (bFromSweep :type Boolean) (SweepResult :type "HitResult Structure (by ref)"))
  (bind _returnvalue (`self.GetOwner` self))
  (if (not (== (`self.GetOwner` OtherActor) _returnvalue))
    (`|ExecutionSequence`
      (:`then_0`
        (`GameplayStatics.ApplyDamage` _returnvalue 0.05 null self)
        (castclass `/Game/Core/BP_Projectile` (`GameplayStatics.GetObjectClass` OtherActor))
        (`self.K2_DestroyActor` OtherActor))
      (:`then_1`
        (`KismetSystemLibrary.DelayUntilNextTick`)
        (`self.K2_DestroyActor`)))))

(fn `UserConstructionScript`
  (`parent.UserConstructionScript`))