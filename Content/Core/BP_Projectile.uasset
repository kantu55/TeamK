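; BP_Projectile is a damage projectile that expires after DestroyTime and tags its Sphere with "Damage" and its BaseDamage value.
; On sphere overlap it waits a tick, then accepts only a BP_Chara other than its parent actor's owner.
; It applies a fixed negative damage to that character and BaseDamage to the parent's owner, then destroys itself a tick later with a debug print.
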(event `self.ReceiveBeginPlay`
  (set `self.Sphere` (`self.Sphere`))
  (set `ActorComponent.ComponentTags` (`|MakeArray` "Damage" (`KismetStringLibrary.Conv_StringToName` (`KismetStringLibrary.Conv_DoubleToString` (`self.Base Damage`)))) (`self.Sphere`))
  (`KismetSystemLibrary.Delay` (`self.DestroyTime`))
  (`self.K2_DestroyActor`))

(event `self.Sphere.OnComponentBeginOverlap`
  (params (OverlappedComponent :type "PrimitiveComponent Object Reference") (OtherActor :type "Actor Object Reference") (OtherComp :type "PrimitiveComponent Object Reference") (OtherBodyIndex :type Integer) (bFromSweep :type Boolean) (SweepResult :type "HitResult Structure (by ref)"))
  (`KismetSystemLibrary.DelayUntilNextTick`)
  (bind _asbp_chara (cast `/Game/Core/BP_Chara` OtherActor))
  (if (not (== OtherActor (`self.GetOwner` (`self.GetParentActor` self))))
    (`GameplayStatics.ApplyDamage` _asbp_chara -1.0)
    (`GameplayStatics.ApplyDamage` (`self.GetOwner` (`self.GetParentActor` self)) (`self.Base Damage`) null self)
    (`KismetSystemLibrary.DelayUntilNextTick`)
    (`KismetSystemLibrary.PrintString` "Damage")
    (`self.K2_DestroyActor`)))

(fn `UserConstructionScript`)