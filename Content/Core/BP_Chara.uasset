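; BP_Chara is a side-view fighter character, locked to the YZ plane, that performs one of five input-selected data-asset actions.
; Action starts a Tick-timed Charge, Attack, Delay state machine, with the asset driving pose, velocity, effects, sound and optional thrown actor.
; Attacks apply damage through a debug-drawn sphere overlap.
; Positive or Tukkomi-projectile damage adds "Wara" points toward a finish call; other damage causes knockback.
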(event `self.ReceiveBeginPlay`)

(event `self.ReceiveTick`
  (params (DeltaSeconds :type "Float (single-precision)"))
  (bind (_returnvalue_x _returnvalue_y _returnvalue_z) (`KismetMathLibrary.BreakVector` (`self.K2_GetActorLocation`)))
  (bind _scene (`self.Scene`))
  (bind _returnvalue (`SceneComponent.K2_GetComponentLocation` _scene))
  (bind (_size _location _damage) (break `/Game/Core/ST_CollisionData` (`|GetArrayItem` (`/Game/Core/BP_PDA_Action.CollisionData` (`self.SelectDataAsset`)))))
  (bind (_x _y) (`KismetMathLibrary.BreakVector2D` _location))
  (`|ExecutionSequence`
    (:`then_0`
      (bind _output_get (set `self.Timecount` (+ (stale _output_get) DeltaSeconds)))
      (if (> (`self.Timecount`) (`self.Limit`))
        (set `self.Timecount` 0.0)
        (switch `/Game/Core/E_CharaState` (`self.State`)
          (:`NewEnumerator0`
            (`self.Attack`))
          (:`NewEnumerator1`
            (`self.Delay`))
          (:`NewEnumerator2`
            (`self.NewFunction` "/Game/Effects/Materials/M_OrverLay_Inst1.M_OrverLay_Inst1" :!label _label)
            (`self.ActionEnd`))
          (:`NewEnumerator3`
            (goto _label)))
        (elif (`|EnumEquality` (`self.State`) "NewEnumerator1")
          (if (`self.f`)
            (`SceneComponent.K2_SetRelativeLocation` (`self.Scene`) (0.0 0.0 0.0) false false)
            (`SceneComponent.K2_AddLocalOffset` _scene (`KismetMathLibrary.MakeVector` _x 0.0 _y) false false)
            (`KismetSystemLibrary.DrawDebugSphere` _returnvalue _size 12 (struct :`R` 1.0 :`G` 0.113322 :`A` 1.0))
            (`KismetSystemLibrary.PrintString` (`KismetStringLibrary.Conv_VectorToString` _returnvalue))
            (bind _outactors (`KismetSystemLibrary.SphereOverlapActors` _returnvalue _size (`|MakeArray` "ObjectTypeQuery3" "ObjectTypeQuery7" :!type "EObjectTypeQuery Enum") "BP_Chara_C" (`|MakeArray` self :!type "Actor Object Reference")))
            (for _array_element _outactors
              (bind _asbp_chara (cast `/Game/Core/BP_Chara` _array_element))
              (if (not (== _asbp_chara self))
                (`self.HIt` _damage _asbp_chara)
                (set `self.f` true)))))))
    (:`then_1`
      (if (`self.Auto`)
        _))
    (:`then_3`
      (`self.K2_SetActorLocation` (`KismetMathLibrary.MakeVector` 0.0 _returnvalue_y _returnvalue_z)))))

(event `EnhancedInput|/Game/Core/Input/IA_Axis`
  (params (ActionValue :type "Vector2D Structure") (ElapsedSeconds :type "Float (double-precision)") (TriggeredSeconds :type "Float (double-precision)") (InputAction :type "InputAction Object Reference" :default "/Game/Core/Input/IA_Axis.IA_Axis"))
  (:`Triggered`
    (set `self.InputDirection` ActionValue)))

(event `Key|Four`
  (params (Key :type "Key Structure")))

(event `Action`
  (set `self.ActionSelect` false)
  (`/Engine/EditorBlueprintResources/StandardMacros.IsValid` (`self.SelectDataAsset`)
    (:`Is Valid`
      (`self.Charge`)
      (`self.NewFunction` "/Game/Effects/Materials/M_OrverLay.M_OrverLay"))))

(event `self.Mesh.OnComponentBeginOverlap`
  (params (OverlappedComponent :type "PrimitiveComponent Object Reference") (OtherActor :type "Actor Object Reference") (OtherComp :type "PrimitiveComponent Object Reference") (OtherBodyIndex :type Integer) (bFromSweep :type Boolean) (SweepResult :type "HitResult Structure (by ref)")))

(event `Attack`
  (bind _selectdataasset (`self.SelectDataAsset`))
  (bind _spawnthrowactor (`/Game/Core/BP_PDA_Action.SpawnThrowActor` _selectdataasset))
  (set `self.State` "NewEnumerator1")
  (`|ExecutionSequence`
    (:`then_1`
      (if (`KismetSystemLibrary.IsValidClass` _spawnthrowactor)
        (bind _returnvalue (`|SpawnActorFromClass` _spawnthrowactor (`KismetMathLibrary.MakeTransform` (`self.K2_GetActorLocation`) (`self.K2_GetActorRotation`)) "Undefined" "MultiplyWithRoot" null null))
        (`self.SetOwner` _returnvalue self)))
    (:`then_2`
      (`self.ChangePose` (`/Game/Core/BP_PDA_Action.PoseAssetName_Attack` _selectdataasset))
      (bind _returnvalue_2 (`KismetSystemLibrary.LoadAsset_Blocking` (`/Game/Core/BP_PDA_Action.NS_Attack` _selectdataasset)))
      (bind _asniagara_system (cast `NiagaraSystem` _returnvalue_2))
      (`NiagaraFunctionLibrary.SpawnSystemAtLocation` _asniagara_system (`SceneComponent.K2_GetComponentLocation` (`self.CapsuleComponent`))))
    (:`then_3`
      (set `self.Limit` (`/Game/Core/BP_PDA_Action.DelayTime_Attack` _selectdataasset))
      (`self.DestroyCollision`))
    (:`then_4`
      (`GameplayStatics.PlaySoundAtLocation` (`/Game/Core/BP_PDA_Action.SoundCue_Attack` _selectdataasset) (`self.K2_GetActorLocation`) (struct) 1.0 1.0 0.0 null null null null))
    (:`then_5`
      (`self.MoveFunc` (`/Game/Core/BP_PDA_Action.MoveVector_Attack` _selectdataasset)))))

(event `Charge`
  (bind _selectdataasset (`self.SelectDataAsset`))
  (set `self.State` "NewEnumerator0")
  (`|ExecutionSequence`
    (:`then_0`
      (`self.MoveFunc` (`/Game/Core/BP_PDA_Action.MoveVector_Charge` _selectdataasset) (`/Game/Core/BP_PDA_Action.FlyVel` _selectdataasset)))
    (:`then_1`
      (`self.ChangePose` (`/Game/Core/BP_PDA_Action.PoseAssetName_Charge` _selectdataasset)))
    (:`then_2`
      (set `self.Limit` (`/Game/Core/BP_PDA_Action.DelayTime_Charge` _selectdataasset)))
    (:`then_3`
      (`GameplayStatics.PlaySoundAtLocation` (`/Game/Core/BP_PDA_Action.SoundCue_Charge` _selectdataasset) (`self.K2_GetActorLocation`) (struct) 1.0 1.0 0.0 null null null null))))

(event `self.ReceiveAnyDamage`
  (params (Damage :type "Float (single-precision)") (DamageType :type "DamageType Object Reference") (InstigatedBy :type "Controller Object Reference") (DamageCauser :type "Actor Object Reference"))
  (if (== (`GameplayStatics.GetObjectClass` DamageCauser) "/Game/Core/BP_ThrowObject_Tukkomi.BP_ThrowObject_Tukkomi_C")
    (set `self.Point` (`KismetMathLibrary.FClamp` (+ (`self.Point`) Damage) 0.0 1.1) :!label _label_2)
    (`self.GetWara` Damage)
    (if (>= (`self.Point`) (`self.WaraMaxPoint`))
      (`self.Fnish`))
    (elif (> Damage 0.0)
      (goto _label_2)
      (else
        (`self.Damage` 0.5)))))

(event `HIt`
  (params (da :type "Float (double-precision)") (NewParam :type "Object Object Reference"))
  (bind _asactor (cast `Actor` NewParam))
  (`GameplayStatics.ApplyDamage` _asactor da)
  (bind _outactors (`GameplayStatics.GetAllActorsOfClass` "BP_Chara_C"))
  (for _array_element _outactors
    (if (not (== _array_element _asactor))
      (`GameplayStatics.ApplyDamage` _asactor -1.0))))

(event `Damage`
  (params (Limit :type "Float (double-precision)"))
  (set `self.State` "NewEnumerator3")
  (set `self.Limit` Limit)
  (set `self.Timecount` 0.0)
  (`self.Move` (0.0 200.0))
  (`self.ChangePose` "/Game/PoseAssets/PA_Yarare_01_Zukkoke_A.PA_Yarare_01_Zukkoke_A")
  (`self.NewFunction` "/Game/Effects/Materials/M_OrverLayDamage.M_OrverLayDamage")
  (`NiagaraFunctionLibrary.SpawnSystemAttached` "/Game/VFX/Star/NS_Hit_Particle_002.NS_Hit_Particle_002" null "None" (`self.K2_GetActorLocation`) (struct) "KeepRelativeOffset"))

(event `Delay`
  (set `self.State` "NewEnumerator2")
  (set `self.Limit` (`/Game/Core/BP_PDA_Action.DelayTime_Delay` (`self.SelectDataAsset`))))

(event `Key|Five`
  (params (Key :type "Key Structure")))

(event `Key|Gamepad_FaceButton_Right`
  (params (Key :type "Key Structure")))

(event `EnhancedInput|/Game/Core/Input/IA_Action_1`
  (params (ActionValue :type Boolean) (ElapsedSeconds :type "Float (double-precision)") (TriggeredSeconds :type "Float (double-precision)") (InputAction :type "InputAction Object Reference" :default "/Game/Core/Input/IA_Action_1.IA_Action_1"))
  (:`Started`
    (set `self.SelectDataAsset` (`|GetArrayItem` (`self.ActionData`)))
    (set `self.ActionSelect` true :!label _label)
    (`self.CharacterRotation`)
    (`self.SelectAction`)))

(event `EnhancedInput|/Game/Core/Input/IA_Action_2`
  (params (ActionValue :type Boolean) (ElapsedSeconds :type "Float (double-precision)") (TriggeredSeconds :type "Float (double-precision)") (InputAction :type "InputAction Object Reference" :default "/Game/Core/Input/IA_Action_2.IA_Action_2"))
  (:`Started`
    (set `self.SelectDataAsset` (`|GetArrayItem` (`self.ActionData`) 1))
    (goto _label)))

(event `EnhancedInput|/Game/Core/Input/IA_Action_3`
  (params (ActionValue :type Boolean) (ElapsedSeconds :type "Float (double-precision)") (TriggeredSeconds :type "Float (double-precision)") (InputAction :type "InputAction Object Reference" :default "/Game/Core/Input/IA_Action_3.IA_Action_3"))
  (:`Started`
    (set `self.SelectDataAsset` (`|GetArrayItem` (`self.ActionData`) 2))
    (goto _label)))

(event `EnhancedInput|/Game/Core/Input/IA_Action_4`
  (params (ActionValue :type Boolean) (ElapsedSeconds :type "Float (double-precision)") (TriggeredSeconds :type "Float (double-precision)") (InputAction :type "InputAction Object Reference" :default "/Game/Core/Input/IA_Action_4.IA_Action_4"))
  (:`Triggered`
    (set `self.SelectDataAsset` (`|GetArrayItem` (`self.ActionData`) 3))
    (goto _label)))

(event `EnhancedInput|/Game/Core/Input/IA_Action_5`
  (params (ActionValue :type Boolean) (ElapsedSeconds :type "Float (double-precision)") (TriggeredSeconds :type "Float (double-precision)") (InputAction :type "InputAction Object Reference" :default "/Game/Core/Input/IA_Action_5.IA_Action_5"))
  (:`Triggered`
    (set `self.SelectDataAsset` (`|GetArrayItem` (`self.ActionData`) 4))
    (goto _label)))

(fn `ActionEnd`
  (set `self.InputDirection` (0.0 0.0))
  (set `self.State` "NewEnumerator4")
  (`self.NewFunction` "/Game/Effects/Materials/M_OrverLay_Inst1.M_OrverLay_Inst1")
  (`self.EndAction`))

(fn `CharacterRotation`
  (if (`self.WasStickInput`)
    (if (`KismetMathLibrary.NearlyEqual_FloatFloat` (+ (.y (`self.GetActorForwardVector`)) (`KismetMathLibrary.BreakVector2D` (`self.InputDirection`))) 1.0 9.0)
      (`self.K2_SetActorRotation` self (`KismetMathLibrary.MakeRotator` 0.0 0.0 (`KismetMathLibrary.SelectFloat` 90.0 -90.0 (> (`KismetMathLibrary.BreakVector2D` (`self.InputDirection`)) 0.0))) false))))

(fn `MoveFunc`
  (params (InputPin :type "Vector2D Structure") (Condition :type Boolean))
  (bind (_x _y) (`KismetMathLibrary.BreakVector2D` InputPin))
  (bind (_x_2 _y_2) (`KismetMathLibrary.BreakVector2D` InputPin))
  (bind _charactermovement (`self.CharacterMovement`))
  (bind _charactermovement_2 (`self.CharacterMovement`))
  (bind _charactermovement_3 (`self.CharacterMovement`))
  (bind (_x_3 _y_3) (`KismetMathLibrary.BreakVector2D` (`self.InputDirection`)))
  (`CharacterMovementComponent.SetMovementMode` (`self.CharacterMovement`) "MOVE_Falling" 0)
  (`self.K2_AddActorWorldOffset` (0.0 0.0 1.0))
  (if (`|EnumEquality` (`self.State`) "NewEnumerator1")
    (set `MovementComponent.Velocity` (+ (`MovementComponent.Velocity` _charactermovement_3) (`KismetMathLibrary.MakeVector` 0.0 (* _x (`KismetMathLibrary.SelectFloat` 1.0 -1.0 (> (.y (`self.GetActorForwardVector`)) 0.0))) _y)) _charactermovement_3)
    (elif Condition
      (set `MovementComponent.Velocity` (+ (`MovementComponent.Velocity` _charactermovement) (`KismetMathLibrary.MakeVector` 0.0 (* (+ (* (`KismetMathLibrary.FClamp` _x_3) 500.0) _x_2) (`KismetMathLibrary.SelectFloat` 1.0 -1.0 (> (.y (`self.GetActorForwardVector`)) 0.0))) (+ (* (`KismetMathLibrary.FClamp` _y_3) 500.0) _y_2))) _charactermovement)
      (else
        (set `MovementComponent.Velocity` (+ (`MovementComponent.Velocity` _charactermovement_2) (`KismetMathLibrary.MakeVector` 0.0 (`KismetMathLibrary.BreakVector2D` (* (0.0 0.0) (`KismetMathLibrary.SelectFloat` 1.0 -1.0 (> (.y (`self.GetActorForwardVector`)) 0.0)))))) _charactermovement_2)))))

(fn `NewFunction`
  (params (NewOverlayMaterial :type "MaterialInterface Object Reference"))
  (`MeshComponent.SetOverlayMaterial` (`self.Mesh`) NewOverlayMaterial))

(fn `UserConstructionScript`)

(fn `WasStickInput`
  (returns (ReturnValue :type Boolean))
  (bind _x (`KismetMathLibrary.BreakVector2D` (`self.InputDirection`)))
  (return (or (> _x 0.2) (> -0.2 _x))))