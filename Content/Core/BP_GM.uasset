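; BP_GM is a manager for a two-player battle that drives the battle UI with a countdown and each player's gauge.
; BeginPlay creates WBP_BattleUI and binds both player pawns' GetWara events, which feed the Wara value into the matching gauge.
; Tick counts down LimitTimer and shows it as whole seconds, with no handling at zero.
; An unconnected chain for creating players and spawning and possessing BP_Chara pawns never runs.
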(event `self.ReceiveBeginPlay`
  (set `self.LimitTimer` 99.0)
  (bind _returnvalue (`|CreateWidget` "/Game/Core/UI/WBP_BattleUI.WBP_BattleUI_C"))
  (bind _output_get (set `self.BattleUI` _returnvalue))
  (`UserWidget.AddToViewport` _output_get 0)
  (bind _output_get_2 (set `self.Player` (`GameplayStatics.GetPlayerPawn` 0)))
  (bind _asbp_chara (cast `/Game/Core/BP_Chara` _output_get_2))
  (add `/Game/Core/BP_Chara.GetWara` _asbp_chara (delegate `damagePlayer1`))
  (bind _output_get_3 (set `self.Player` (`GameplayStatics.GetPlayerPawn` 1)))
  (bind _asbp_chara_2 (cast `/Game/Core/BP_Chara` _output_get_3))
  (add `/Game/Core/BP_Chara.GetWara` _asbp_chara_2 (delegate `damagePlayer2`)))

(event `damagePlayer1`
  (params (Wara :type "Float (double-precision)"))
  (bind _battleui (`self.BattleUI`)
    (:`then`
      (`/Game/Core/UI/WBP_BattleUI.SetPlayerGaugePercent` _battleui 0 Wara))
    (:`else`)))

(event `damagePlayer2`
  (params (Wara :type "Float (double-precision)"))
  (bind _battleui (`self.BattleUI`)
    (:`then`
      (`/Game/Core/UI/WBP_BattleUI.SetPlayerGaugePercent` _battleui 1 Wara))
    (:`else`)))

(event `self.ReceiveTick`
  (params (DeltaSeconds :type "Float (single-precision)"))
  (bind _output_get (set `self.LimitTimer` (- (`self.LimitTimer`) DeltaSeconds)))
  (bind _battleui (`self.BattleUI`)
    (:`then`
      (`/Game/Core/UI/WBP_BattleUI.SetTimer` _battleui (`KismetMathLibrary.FTrunc` _output_get)))
    (:`else`)))

(fn `UserConstructionScript`)