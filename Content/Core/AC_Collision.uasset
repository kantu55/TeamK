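; AC_Collision is a collision component that detects BP_Chara actors within a sphere around its world location.
; Each tick it runs a sphere overlap filtered to BP_Chara and calls Orver with Da and each hit character, excluding its owner.
; It also prints debug text and draws the sphere every tick, and retains a disconnected sphere trace.
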(event `self.ReceiveBeginPlay`)

(event `self.ReceiveTick`
  (params (DeltaSeconds :type "Float (single-precision)"))
  (bind _returnvalue (`self.K2_GetComponentLocation`))
  (`KismetSystemLibrary.PrintString` "Hello")
  (`KismetSystemLibrary.PrintString` (`KismetStringLibrary.Conv_VectorToString` _returnvalue))
  (`KismetSystemLibrary.DrawDebugSphere` _returnvalue (`self.Sphere Radius`) 12 (struct :`R` 0.109285 :`B` 1.0 :`A` 1.0) 5.0 5.0)
  (bind _outactors (`KismetSystemLibrary.SphereOverlapActors` _returnvalue (`self.Sphere Radius`) (`|MakeArray` "ObjectTypeQuery3" "ObjectTypeQuery7" :!type "EObjectTypeQuery Enum") "/Game/Core/BP_Chara.BP_Chara_C"))
  (for _array_element _outactors
    (bind _asbp_chara (cast `/Game/Core/BP_Chara` _array_element))
    (if (not (== _asbp_chara (`self.GetOwner`)))
      (`self.Orver` (`self.Da`) _asbp_chara)))
  (`KismetSystemLibrary.DelayUntilNextTick`)
  (`KismetSystemLibrary.DelayUntilNextTick`))